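; Ghost actor that slowly homes in on the first player character.
; Each tick it eases its AllowTransform component's rotation toward the player's capsule with RInterpTo, then moves that component along its local forward axis at constant speed.
; The gradual turn gives a curved pursuit, and movement is unswept, so geometry does not block it.
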(event EventTick
  (params (DeltaSeconds :type Float%20%28single-precision%29))
  (bind _allowtransform (Variables|Default|GetAllowTransform))
  (Variables|Default|SetDelta%20seconds DeltaSeconds)
  (Transformation|SetWorldRotation (Variables|Default|GetAllowTransform) (Math|Interpolation|RInterpTo (Transformation|GetWorldRotation _allowtransform) (Math|Rotator|FindLookatRotation (Transformation|GetWorldLocation _allowtransform) (Transformation|GetWorldLocation (Variables|/Script/Engine.Character|GetCapsuleComponent (Game|GetPlayerCharacter 0)))) (Variables|Default|GetDelta%20seconds) 1.5) false)
  (Transformation|AddLocalOffset (Variables|Default|GetAllowTransform) (* (Math|Vector|MakeVector 75.0 0.0 0.0) (Variables|Default|GetDelta%20seconds)) false))

(fn ConstructionScript)